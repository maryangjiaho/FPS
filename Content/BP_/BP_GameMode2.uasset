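; Wave-survival game mode that spawns escalating zombie waves at random target points, ending with a single final enemy.
; A wave ID selects enemy class and count, while a polling timer detects cleared waves, restores player health and starts the next after a delay.
; A separate timer respawns a rifle ammo pickup after the previous one is destroyed.
; Once the final enemy is gone, a Success widget appears with UI-only input.
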(event `UpdataEmpty`
  (switch `int` (`self.ID`) :!label _label
    (:`0`
      (for _ (range 6)
        (`AIBlueprintHelperLibrary.SpawnAIFromClass` "/Game/FPS_Game/Blueprints/Bonus/AI/Zombie/Empty/1.1_C" null (`self.SpawnLocation`))
        (`self.Updata`)))
    (:`1`
      (for _ (range 6)
        (`AIBlueprintHelperLibrary.SpawnAIFromClass` "/Game/FPS_Game/Blueprints/Bonus/AI/Zombie/Empty/1_2.1_2_C" null (`self.SpawnLocation`))
        (`self.Updata`)))
    (:`2`
      (for _ (range 7)
        (`AIBlueprintHelperLibrary.SpawnAIFromClass` "/Game/FPS_Game/Blueprints/Bonus/AI/Zombie/Empty/2.2_C" null (`self.SpawnLocation`))
        (`self.Updata`)))
    (:`3`
      (for _ (range 7)
        (`AIBlueprintHelperLibrary.SpawnAIFromClass` "/Game/FPS_Game/Blueprints/Bonus/AI/Zombie/Empty/2_2.2_2_C" null (`self.SpawnLocation`))
        (`self.Updata`)))
    (:`4`
      (for _ (range 8)
        (`AIBlueprintHelperLibrary.SpawnAIFromClass` "/Game/FPS_Game/Blueprints/Bonus/AI/Zombie/Empty/3.3_C" null (`self.SpawnLocation`))
        (`self.Updata`)))
    (:`5`
      (for _ (range 8)
        (`AIBlueprintHelperLibrary.SpawnAIFromClass` "/Game/FPS_Game/Blueprints/Bonus/AI/Zombie/Empty/3_2.3_2_C" null (`self.SpawnLocation`))
        (`self.Updata`)))
    (:`6`
      (for _ (range 9)
        (`AIBlueprintHelperLibrary.SpawnAIFromClass` "/Game/FPS_Game/Blueprints/Bonus/AI/Zombie/Empty/4.4_C" null (`self.SpawnLocation`))
        (`self.Updata`)))
    (:`7`
      (for _ (range 9)
        (`AIBlueprintHelperLibrary.SpawnAIFromClass` "/Game/FPS_Game/Blueprints/Bonus/AI/Zombie/Empty/4_2.4_2_C" null (`self.SpawnLocation`))
        (`self.Updata`)))
    (:`8`
      (for _ (range 10)
        (`AIBlueprintHelperLibrary.SpawnAIFromClass` "/Game/FPS_Game/Blueprints/Bonus/AI/Zombie/Empty/5.5_C" null (`self.SpawnLocation`))
        (`self.Updata`)))
    (:`9`
      (bind _returnvalue (`AIBlueprintHelperLibrary.SpawnAIFromClass` "/Game/FPS_Game/Blueprints/Bonus/AI/Zombie/Empty/6.6_C" null (`self.SpawnLocation`)))
      (set `self.NewVar_0` _returnvalue)
      (bind _returnvalue_2 (`KismetSystemLibrary.K2_SetTimerDelegate` (delegate `自定义事件_2`) 0.1 true))
      (set `self.NewVar_1` _returnvalue_2))))

(event `self.ReceiveBeginPlay`
  (bind _returnvalue (`GameplayStatics.GetPlayerController` 0))
  (`|ExecutionSequence`
    (:`then_0`
      (bind _outactors (`GameplayStatics.GetAllActorsOfClass` "/Script/Engine.TargetPoint"))
      (set `self.SpawnPoint` _outactors)
      (goto _label))
    (:`then_1`
      (bind _outactors_2 (`GameplayStatics.GetAllActorsOfClass` "/Game/FPS_Game/Blueprints/PickUps/NewBlueprint.NewBlueprint_C" :!label _label_2))
      (bind _returnvalue_2 (`KismetSystemLibrary.K2_SetTimerDelegate` (delegate `自定义事件_1`) 20.0 true))
      (set `self.T` _returnvalue_2))
    (:`then_2`
      (set `PlayerController.bShowMouseCursor` false _returnvalue)
      (`WidgetBlueprintLibrary.SetInputMode_GameOnly` _returnvalue))))

(event `Updata`
  ;[1 1 1] 更新怪物类型
  (bind _returnvalue (`KismetSystemLibrary.K2_SetTimerDelegate` (delegate `自定义事件_0`) 0.1 true))
  (set `self.Timer` _returnvalue))

(event `UpdataAmmo`
  (`/Engine/EditorBlueprintResources/StandardMacros.IsValid` (`self.Ammo`)
    (:`Is Not Valid`
      (goto _label_2))))

(event `自定义事件_0`
  ;[1 1 1] 更新怪物类型
  (if (== (`self.UpdataEm`) 0)
    (`KismetSystemLibrary.K2_ClearAndInvalidateTimerHandle` (`self.Timer`))
    (`/Engine/EditorBlueprintResources/StandardMacros.IncrementInt` (`self.ID`)
      (:`  `
        (set `/Game/FPS_Game/Blueprints/BP_CharacterBase.HealthCurrent` 5.0 (cast `/Game/FPS_Game/Blueprints/BP_CharacterBase` (`Controller.K2_GetPawn` (`GameplayStatics.GetPlayerController` 0)) :!pure true))
        (`KismetSystemLibrary.Delay` 10.0)
        (`self.UpdataEmpty`)))))

(event `自定义事件_1`
  (bind _returnvalue (`|SpawnActorFromClass` "/Game/FPS_Game/Blueprints/PickUps/BPC_AmmoRifle.BPC_AmmoRifle_C" (`KismetMathLibrary.MakeTransform` (`self.K2_GetActorLocation` (`|GetArrayItem` (stale `self.ReceiveBeginPlay` _outactors_2)))) "Undefined" "OverrideRootScale" null null))
  (bind _output_get (set `self.Ammo` _returnvalue))
  (set `/Game/FPS_Game/Blueprints/PickUps/BASE/BP_AmmoPickUp_BASE.AmmoToAdd` 25 _output_get)
  (`KismetSystemLibrary.K2_ClearAndInvalidateTimerHandle` (`self.T`))
  (add `/Game/FPS_Game/Blueprints/PickUps/BASE/BP_AmmoPickUp_BASE.Dest` _output_get (delegate `Dest_事件_0`)))

(event `Dest_事件_0`
  (set `self.Ammo` null)
  (`self.UpdataAmmo`))

(event `自定义事件_2`
  (bind _returnvalue (`GameplayStatics.GetPlayerController` 0))
  (`/Engine/EditorBlueprintResources/StandardMacros.IsValid` (`self.NewVar_0`)
    (:`Is Not Valid`
      (`KismetSystemLibrary.K2_ClearAndInvalidateTimerHandle` (`self.NewVar_1`))
      (bind _returnvalue_2 (`|CreateWidget` "/Game/BP_/Success.Success_C"))
      (`UserWidget.AddToViewport` _returnvalue_2 0)
      (set `PlayerController.bShowMouseCursor` true _returnvalue)
      (`WidgetBlueprintLibrary.SetInputMode_UIOnlyEx` _returnvalue null))))

(fn `SpawnLocation`
  (returns (ReturnValue1 :type "Vector Structure"))
  (return (`self.K2_GetActorLocation` (`|GetArrayItem` (`self.SpawnPoint`) (`KismetMathLibrary.RandomInteger` 2)))))

(fn `UpdataEm`
  (returns (ReturnValue :type Integer))
  (locals (Int :type Integer :default 0))
  (bind _outactors (`GameplayStatics.GetAllActorsOfClass` "/Game/FPS_Game/Blueprints/Bonus/AI/Zombie/BP_AI_CharZombie.BP_AI_CharZombie_C"))
  (set `local.Int` (`KismetArrayLibrary.Array_Length` _outactors))
  (return (`local.Int`)))

(fn `UserConstructionScript`)